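; Start/finish line actor for the AI race mode, using a box trigger to drive race and lap progress.
; BeginPlay caches the first player's VehiclePlayerController and the AIGameMode.
; The first overlap starts the lap and race; later overlaps increment the game mode's completed laps, then either roll into a new lap or end the race at the required count.
; The overlap does not check which actor entered.
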(event `self.ReceiveBeginPlay`
  (bind _asvehicle_player_controller (cast `/Game/VehicleTemplate/Blueprints/VehiclePlayerController` (`GameplayStatics.GetPlayerController` 0)))
  (set `self.As Vehicle Player Controller` _asvehicle_player_controller)
  (bind _asaigame_mode (cast `/Game/VehicleTemplate/Blueprints/AIGameMode` (`GameplayStatics.GetGameMode`)))
  (set `self.As AIGame Mode` _asaigame_mode))

(event `self.Box.OnComponentBeginOverlap`
  (params (OverlappedComponent :type "PrimitiveComponent Object Reference") (OtherActor :type "Actor Object Reference") (OtherComp :type "PrimitiveComponent Object Reference") (OtherBodyIndex :type Integer) (bFromSweep :type Boolean) (SweepResult :type "HitResult Structure (by ref)"))
  (bind _as_vehicle_player_controller (`self.As Vehicle Player Controller`))
  (bind _as_aigame_mode (`self.As AIGame Mode`))
  (if (`self.RaceStarted`)
    (bind _result (`/Engine/EditorBlueprintResources/StandardMacros.IncrementInt` (`/Game/VehicleTemplate/Blueprints/AIGameMode.LapsCompleted` _as_aigame_mode))
      (:`  `
        (if (== _result (`/Game/VehicleTemplate/Blueprints/AIGameMode.LapsRequired` _as_aigame_mode))
          (`/Game/VehicleTemplate/Blueprints/VehiclePlayerController.End Race` _as_vehicle_player_controller)
          (`/Game/VehicleTemplate/Blueprints/VehiclePlayerController.End Lap` _as_vehicle_player_controller)
          (else
            (`/Game/VehicleTemplate/Blueprints/VehiclePlayerController.End Lap` _as_vehicle_player_controller)
            (`/Game/VehicleTemplate/Blueprints/VehiclePlayerController.Start Lap` _as_vehicle_player_controller)
            (`/Game/VehicleTemplate/Blueprints/AIGameMode.UpdateLaps` _as_aigame_mode)))))
    (else
      (`/Game/VehicleTemplate/Blueprints/VehiclePlayerController.Start Lap` _as_vehicle_player_controller)
      (`/Engine/EditorBlueprintResources/StandardMacros.DoOnce` false
        (:`Completed`
          (`/Game/VehicleTemplate/Blueprints/VehiclePlayerController.Start Race` _as_vehicle_player_controller)
          (set `self.RaceStarted` true))))))

(fn `UserConstructionScript`)